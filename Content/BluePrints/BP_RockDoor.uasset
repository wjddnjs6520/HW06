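; BP_RockDoor is a rock door actor that moves between its placed position and an open position far below it.
; BeginPlay stores the starting location as closed and derives the open location by subtracting a fixed vertical offset.
; Open and Close events each restart their own timeline, whose track drives a vector lerp between the two locations, applied without sweep.
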(event `Open`
  (bind (_direction _newtrack_0) (`Timeline|OpenDoor` :!via `PlayFromStart`)
    (:`Update`
      (`self.K2_SetActorLocation` (`KismetMathLibrary.VLerp` (`self.CloseLocation`) (`self.OpenLocation`) _newtrack_0)))))

(event `Close`
  (bind (_direction _newtrack_0) (`Timeline|Timeline` :!via `PlayFromStart`)
    (:`Update`
      (`self.K2_SetActorLocation` (`KismetMathLibrary.VLerp` (`self.CloseLocation`) (`self.OpenLocation`) _newtrack_0)))))

(event `self.ReceiveBeginPlay`
  (bind _output_get (set `self.CloseLocation` (`self.K2_GetActorLocation`)))
  (set `self.OpenLocation` (- _output_get (0.0 0.0 3000.0))))

(fn `UserConstructionScript`)